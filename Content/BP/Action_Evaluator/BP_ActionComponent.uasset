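; Action component that arbitrates gameplay-tagged actions from an input buffer and a queued-action slot, driving state transitions.
; Each tick it evaluates a valid queued action first; otherwise it clears the slot and peeks the fastest buffered input.
; Each evaluation is broadcast; Accept or Interrupt enters the tag's mapped state.
; Buffered input is popped only on Accept, Interrupt or Queue, and its state entries debug-print runtime tags.
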(event EventTick
  (params (DeltaSeconds :type Float%20%28single-precision%29))
  (bind _returnvalue (Class|ActionComponent|GetQueuedActionTag))
  (if (Class|ActionComponent|QueuedActionIsValid (Utilities|Time|GetGameTimeinSeconds))
    (bind _returnvalue_2 (Class|ActionComponent|EvaluateActionBP (Class|ActionComponent|GetQueuedActionTag) (Utilities|Time|GetGameTimeinSeconds)))
    (Class|ActionComponent|BroadcastEvaluationResult (Utilities|Struct|MakeActionDecision (.decision _returnvalue_2) (.reason _returnvalue_2) (.actiontag _returnvalue_2)))
    (if (or (Utilities|Enum|Equal(Enum) (.decision _returnvalue_2) "Accept") (Utilities|Enum|Equal(Enum) (.decision _returnvalue_2) "Interrupt"))
      (bind _returnvalue_3 (Class|ActionComponent|ActionTagtoState _returnvalue))
      (Class|ActionComponent|EnterState _returnvalue_3 _returnvalue (Utilities|Time|GetGameTimeinSeconds))
      (Class|ActionComponent|ClearQueuedAction))
    (else
      (Class|ActionComponent|ClearQueuedAction)
      (bind (_outactiontag _returnvalue_4) (Class|ActionComponent|PeekFastestInput (Utilities|Time|GetGameTimeinSeconds)))
      (if _returnvalue_4
        (bind _returnvalue_5 (Class|ActionComponent|EvaluateActionBP _outactiontag (Utilities|Time|GetGameTimeinSeconds)))
        (Class|ActionComponent|BroadcastEvaluationResult (Utilities|Struct|MakeActionDecision (.decision _returnvalue_5) (.reason _returnvalue_5) (.actiontag _returnvalue_5)))
        (if (Math|Boolean|ORBoolean (Utilities|Enum|Equal(Enum) (.decision _returnvalue_5) "Accept") (Utilities|Enum|Equal(Enum) (.decision _returnvalue_5) "Interrupt") (Utilities|Enum|Equal(Enum) (.decision _returnvalue_5) "Queue"))
          (bind _outactiontag_2 (Class|ActionComponent|PopFastestInput (Utilities|Time|GetGameTimeinSeconds)))
          (if (or (Utilities|Enum|Equal(Enum) (.decision _returnvalue_5) "Accept") (Utilities|Enum|Equal(Enum) (.decision _returnvalue_5) "Interrupt"))
            (bind _returnvalue_6 (Class|ActionComponent|ActionTagtoState _outactiontag_2))
            (Class|ActionComponent|EnterState _returnvalue_6 _outactiontag_2 (Utilities|Time|GetGameTimeinSeconds))
            (for _array_element (Utilities|Array|MakeArray (.RuntimeTags (Utilities|Struct|BreakCurrentState (Variables|Default|GetCurrentState))))
              (Development|PrintString (GameplayTags|GetDebugStringfromGameplayTagContainer _array_element)))))))))