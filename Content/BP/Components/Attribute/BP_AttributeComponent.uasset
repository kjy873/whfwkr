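; BP_AttributeComponent is an attribute component that carries player attributes and upgrades to and from the game instance.
; On BeginPlay it loads upgrades and available upgrades through a MainGameInstance cast, then local player attributes through a BP_GameInstance cast.
; SendToGameInstance writes upgrades and attributes back to BP_GameInstance; available upgrades are only read, never written back.
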(event Custom|SendToGameInstance
  (bind _asbp_game_instance (Utilities|Casting|CastToBP_GameInstance (Game|GetGameInstance)))
  (Class|MainGameInstance|SetUpgrades _asbp_game_instance (Class|AttributeComponent|GetUpgrades))
  (Class|MainGameInstance|SetLocalPlayerAttributes _asbp_game_instance (Class|AttributeComponent|GetAttributes)))

(event EventBeginPlay
  (Utilities|FlowControl|Sequence
    (:then_0
      (bind _asmain_game_instance (Utilities|Casting|CastToMainGameInstance (Game|GetGameInstance)))
      (Class|AttributeComponent|SetUpgrades (Class|MainGameInstance|GetUpgrades _asmain_game_instance))
      (Class|AttributeComponent|SetAvailableUpgrades (Class|MainGameInstance|GetAvailableUpgrades _asmain_game_instance)))
    (:then_1
      (bind _asbp_game_instance (Utilities|Casting|CastToBP_GameInstance (Game|GetGameInstance)))
      (Class|AttributeComponent|SetAttributes (Class|MainGameInstance|GetLocalPlayerAttributes _asbp_game_instance)))))