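; Action component that arbitrates buffered player actions each tick and drives state changes.
; A valid queued action is evaluated first; otherwise it clears the queue and evaluates the fastest buffered input.
; Each decision is broadcast: Accept or Interrupt enters the tag's mapped state, as does Hold for buffered input.
; Queue and Release only consume the input, while other decisions leave it in place.
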(event EventTick
  (params (DeltaSeconds :type Float%20%28single-precision%29))
  (bind _returnvalue (Class|ActionComponent|GetQueuedActionTag))
  (bind _returnvalue_2 (Class|ActionComponent|QueuedActionIsValid (Utilities|Time|GetGameTimeinSeconds)))
  (if _returnvalue_2
    (bind _returnvalue_3 (Class|ActionComponent|EvaluateActionBP (Class|ActionComponent|GetQueuedActionTag) (Utilities|Time|GetGameTimeinSeconds)))
    (Class|ActionComponent|BroadcastEvaluationResult (Utilities|Struct|MakeActionDecision (.decision _returnvalue_3) (.reason _returnvalue_3) (.actiontag _returnvalue_3)))
    (if (or (Utilities|Enum|Equal(Enum) (.decision _returnvalue_3) "Accept") (Utilities|Enum|Equal(Enum) (.decision _returnvalue_3) "Interrupt"))
      (bind _returnvalue_4 (Class|ActionComponent|ActionTagtoState _returnvalue))
      (Class|ActionComponent|EnterState _returnvalue_4 _returnvalue (Utilities|Time|GetGameTimeinSeconds))
      (Class|ActionComponent|ClearQueuedAction))
    (else
      (Class|ActionComponent|ClearQueuedAction)
      (bind (_outactiontag _returnvalue_5) (Class|ActionComponent|PeekFastestInput (Utilities|Time|GetGameTimeinSeconds)))
      (if _returnvalue_5
        (bind _returnvalue_6 (Class|ActionComponent|EvaluateActionBP _outactiontag (Utilities|Time|GetGameTimeinSeconds)))
        (Class|ActionComponent|BroadcastEvaluationResult (Utilities|Struct|MakeActionDecision (.decision _returnvalue_6) (.reason _returnvalue_6) (.actiontag _returnvalue_6)))
        (if (Math|Boolean|ORBoolean (Utilities|Enum|Equal(Enum) (.decision _returnvalue_6) "Accept") (Utilities|Enum|Equal(Enum) (.decision _returnvalue_6) "Interrupt") (Utilities|Enum|Equal(Enum) (.decision _returnvalue_6) "Queue") (Utilities|Enum|Equal(Enum) (.decision _returnvalue_6) "Hold") (Utilities|Enum|Equal(Enum) (.decision _returnvalue_6) "Release"))
          (bind _outactiontag_2 (Class|ActionComponent|PopFastestInput (Utilities|Time|GetGameTimeinSeconds)))
          (if (Math|Boolean|ORBoolean (Utilities|Enum|Equal(Enum) (.decision _returnvalue_6) "Accept") (Utilities|Enum|Equal(Enum) (.decision _returnvalue_6) "Interrupt") (Utilities|Enum|Equal(Enum) (.decision _returnvalue_6) "Hold"))
            (bind _returnvalue_7 (Class|ActionComponent|ActionTagtoState _outactiontag_2))
            (Class|ActionComponent|EnterState _returnvalue_7 _outactiontag_2 (Utilities|Time|GetGameTimeinSeconds))))))))