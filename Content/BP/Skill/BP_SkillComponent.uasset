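; BP_SkillComponent is an actor component that holds the skills available to its owner and activates them by index.
; On BeginPlay it gets the owner's animated mesh via GetAnimatedMeshMessage and caches DT_Skill rows whose OwnerID matches the owner's class.
; ActivateSkillByNum plays the skill's montage on that mesh unless it is locked.
; CanActivate reports the unlocked state, while ActivateSkill is an empty stub.
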(event Custom|ActivateSkillByNum
  (params (SkillNum :type Integer))
  (bind _skilldata (Variables|Default|GetSkillData))
  (bind _output (Utilities|Array|Get(acopy) _skilldata SkillNum))
  (bind (_ownerid _name _displayname _icon _reusablility _montagetoplay _locked) (Utilities|Struct|BreakStructSkillData _output))
  (if (not _locked)
    (Animation|Montage|PlayMontage (Variables|Default|GetMesh) _montagetoplay)))

(event EventBeginPlay
  (bind _output_get (Variables|Default|SetOwner (Components|GetOwner)))
  (bind _animatedmesh (Class|BPICharacterInfo|GetAnimatedMesh(Message) _output_get))
  (Variables|Default|SetMesh _animatedmesh)
  (bind _outrownames (DataTable|GetDataTableRowNames "/Game/BP/Skill/DT_Skill.DT_Skill"))
  (for _array_element _outrownames
    (bind _returnvalue (Utilities|GetDataTableRow "/Game/BP/Skill/DT_Skill.DT_Skill" _array_element)
      (:then
        (if (== (.OwnerID (Utilities|Struct|BreakStructSkillData _returnvalue)) (Utilities|GetClass (Variables|Default|GetOwner)))
          (Utilities|Array|Add :TargetArray (Variables|Default|GetSkillData)))))))

(fn ActivateSkill)

(fn CanActivate
  (params (Dimension%201 :type Integer))
  (return (not (.Locked (Utilities|Struct|BreakStructSkillData (Utilities|Array|Get(acopy) (Variables|Default|GetSkillData) Dimension%201))))))