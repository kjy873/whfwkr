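; Explosive bullet actor that destroys what it touches, except BP_ThirdPersonCharacter.
; On spawn it plays a sound and an unattached fire effect, then destroys itself after a short delay.
; Sphere hit and overlap both fire a radial impulse, spawn explosion effects, and destroy the other actor and the bullet.
; The hit and timeout paths also remove the fire effect, but the overlap path does not.
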(event OnComponentBeginOverlap(Sphere)
  (params (OverlappedComponent :type Primitive%20Component%20Object%20Reference) (OtherActor :type Actor%20Object%20Reference) (OtherComp :type Primitive%20Component%20Object%20Reference) (OtherBodyIndex :type Integer) (bFromSweep :type Boolean) (SweepResult :type Hit%20Result%20Structure%20%28by%20ref%29))
  (bind _location (Collision|BreakHitResult SweepResult))
  (Development|PrintString "overlap")
  (Utilities|Casting|CastToBP_ThirdPersonCharacter OtherActor
    (:CastFailed
      (Class|RadialForceComponent|FireImpulse (Variables|Default|GetRadialForce))
      (Effects|SpawnEmitteratLocation "/Game/StarterContent/Particles/P_Explosion.P_Explosion" _location)
      (Audio|PlaySoundatLocation "/Engine/VREditor/Sounds/UI/Dockable_Window_Close.Dockable_Window_Close" _location "0, 0, 0" 1.0 1.0 0.0 0 0 0 0)
      (Actor|DestroyActor OtherActor)
      (Actor|DestroyActor)
      (Development|PrintString "삭제완"))))

(event OnComponentHit(Sphere)
  (params (HitComponent :type Primitive%20Component%20Object%20Reference) (OtherActor :type Actor%20Object%20Reference) (OtherComp :type Primitive%20Component%20Object%20Reference) (NormalImpulse :type Vector :default "0, 0, 0") (Hit :type Hit%20Result%20Structure%20%28by%20ref%29))
  (bind _location (Collision|BreakHitResult Hit))
  (Utilities|Casting|CastToBP_ThirdPersonCharacter OtherActor
    (:CastFailed
      (Class|RadialForceComponent|FireImpulse (Variables|Default|GetRadialForce))
      (Effects|SpawnEmitteratLocation "/Game/StarterContent/Particles/P_Explosion.P_Explosion" _location)
      (Audio|PlaySoundatLocation "/Engine/VREditor/Sounds/UI/Dockable_Window_Close.Dockable_Window_Close" _location "0, 0, 0" 1.0 1.0 0.0 0 0 0 0)
      (Actor|DestroyActor OtherActor)
      (Actor|DestroyActor)
      (Components|DestroyComponent (stale EventBeginPlay _returnvalue_2))
      (Development|PrintString "삭제완"))))

(event EventBeginPlay
  (bind _returnvalue (Transformation|GetActorLocation))
  (Audio|PlaySoundatLocation "/Game/StarterContent/Audio/Explosion01.Explosion01" _returnvalue "0, 0, 0" 1.0 1.0 0.0 0 0 0 0)
  (bind _returnvalue_2 (Effects|SpawnEmitteratLocation "/Game/StarterContent/Particles/P_Fire.P_Fire" _returnvalue))
  (Utilities|FlowControl|Delay 2.0)
  (Actor|DestroyActor)
  (Components|DestroyComponent _returnvalue_2))

(fn ConstructionScript)