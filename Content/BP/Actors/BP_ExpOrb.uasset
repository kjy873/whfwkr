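; BP_ExpOrb is an experience pickup that flies to its Target and grants a fixed amount of EXP.
; Both trigger areas enable overlaps shortly after spawn.
; HomingArea overlap starts a timeline pushing the orb away from Target, then another homing it toward Target's current location, also restarted by a parallel delay.
; CollectingArea overlap sends Target the EXP message, plays a sound and destroys the orb.
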(event OnComponentBeginOverlap(CollectingArea)
  (params (OverlappedComponent :type Primitive%20Component%20Object%20Reference) (OtherActor :type Actor%20Object%20Reference) (OtherComp :type Primitive%20Component%20Object%20Reference) (OtherBodyIndex :type Integer) (bFromSweep :type Boolean) (SweepResult :type Hit%20Result%20Structure%20%28by%20ref%29))
  (if (== OtherActor (Variables|Default|GetTarget))
    (Class|BPICharacterInfo|AddExpValue(Message) OtherActor 15.0)
    (Audio|PlaySoundatLocation "/Engine/VREditor/Sounds/VR_click1_Cue.VR_click1_Cue" (Transformation|GetActorLocation) "0, 0, 0" 1.0 1.0 0.0 0 0 0 0)
    (Actor|DestroyActor)))

(event OnComponentBeginOverlap(HomingArea)
  (params (OverlappedComponent :type Primitive%20Component%20Object%20Reference) (OtherActor :type Actor%20Object%20Reference) (OtherComp :type Primitive%20Component%20Object%20Reference) (OtherBodyIndex :type Integer) (bFromSweep :type Boolean) (SweepResult :type Hit%20Result%20Structure%20%28by%20ref%29))
  (bind _returnvalue (Transformation|GetActorLocation))
  (bind _target (Variables|Default|GetTarget))
  (if (== OtherActor _target)
    (Variables|Default|SetPushWhenOverlapped (+ _returnvalue (* (- _returnvalue (Transformation|GetActorLocation _target)) 0.5)))
    (Utilities|FlowControl|Sequence
      (:then_0
        (bind _value (Timeline|AwayFromPlayer PlayFromStart)
          (:Update
            (Transformation|SetActorLocation (Math|Vector|Lerp(Vector) (Transformation|GetActorLocation) (Variables|Default|GetPushWhenOverlapped) _value) false false))
          (:Finished
            (bind _value_2 (Timeline|HomeToPlayer PlayFromStart)
              (:Update
                (Transformation|SetActorLocation (Math|Vector|Lerp(Vector) (Transformation|GetActorLocation) (Transformation|GetActorLocation _target) _value_2) false false))))))
      (:then_1
        (Utilities|FlowControl|Delay 0.4)
        (Audio|Components|Audio|Stop (Variables|Default|GetHomeToPlayer))
        (Timeline|HomeToPlayer PlayFromStart)))))

(event EventBeginPlay
  (Utilities|FlowControl|Delay 0.2)
  (Variables|/Script/Engine.PrimitiveComponent|SetbGenerateOverlapEvents (Variables|Default|GetHomingArea) true)
  (Variables|/Script/Engine.PrimitiveComponent|SetbGenerateOverlapEvents (Variables|Default|GetCollectingArea) true))

(event Collision|EventActorBeginOverlap
  (params (OtherActor :type Actor%20Object%20Reference)))

(event EventTick
  (params (DeltaSeconds :type Float%20%28single-precision%29)))

(fn ConstructionScript)