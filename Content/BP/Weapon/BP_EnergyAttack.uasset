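; BP_EnergyAttack is a weapon attack actor that, in this graph, only tracks its owning character and prints debug messages.
; On BeginPlay it prints the OwnerCharacter's name if set, otherwise it stores the Instigator cast to BP_GameCharacter as the owner.
; It also prints a message when destroyed.
; Overlap and Tick are disabled placeholders, and the construction script only calls the parent, so no movement or damage logic appears here.
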(event EventBeginPlay
  (Utilities|IsValid (Variables|Default|GetOwnerCharacter)
    (:Is%20Valid
      (Development|PrintString (Utilities|GetDisplayName (Variables|Default|GetOwnerCharacter))))
    (:Is%20Not%20Valid
      (bind _asbp_game_character (Utilities|Casting|CastToBP_GameCharacter (Game|GetInstigator)))
      (Variables|Default|SetOwnerCharacter _asbp_game_character))))

(event Collision|EventActorBeginOverlap
  (params (OtherActor :type Actor%20Object%20Reference))
  (|CallParentFunction OtherActor) ; 지금 이 노드는 비활성 상태입니다. \n핀을 끌어서 다른 노드를 연결하면 활성화됩니다.
)

(event EventTick
  (params (DeltaSeconds :type Float%20%28single-precision%29))
  (|CallParentFunction DeltaSeconds) ; 지금 이 노드는 비활성 상태입니다. \n핀을 끌어서 다른 노드를 연결하면 활성화됩니다.
)

(event EventDestroyed
  (Development|PrintString "Destroyed"))

(fn ConstructionScript
  (|CallParentFunction))