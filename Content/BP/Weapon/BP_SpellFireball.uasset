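; Fireball spell projectile that charges while growing, then launches on ProjectileLaunch and deals fire damage to actors other than its owner.
; A timeline scales the actor, Niagara effect and launch speed together until launch stops it.
; Launch detaches it, while a looping timer compounds velocity and homing acceleration.
; Impact hides the effect and briefly enables an explosion collider for one-third damage before destruction.
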(event OnComponentBeginOverlap(Sphere)
  (params (OverlappedComponent :type Primitive%20Component%20Object%20Reference) (OtherActor :type Actor%20Object%20Reference) (OtherComp :type Primitive%20Component%20Object%20Reference) (OtherBodyIndex :type Integer) (bFromSweep :type Boolean) (SweepResult :type Hit%20Result%20Structure%20%28by%20ref%29))
  (if (!= OtherActor (Variables|Default|GetOwnerCharacter))
    (Audio|PlaySoundatLocation "/Game/SFX/Spell/Fireball/Impact/fire-magic-6947_Cue.fire-magic-6947_Cue" (Transformation|GetActorLocation) "0, 0, 0" 1.0 1.0 0.0 "/Game/SFX/DefaultAttanuation.DefaultAttanuation" 0 0 0)
    (Class|BPICharacterInfo|RecvDamage(Message) OtherActor (Variables|Default|GetDamageValue) "(TagName=\"DamageType.Fire\")" (Variables|Default|GetOwnerCharacter))
    (Utilities|HitFireBall)))

(event OnComponentHit(Sphere)
  (params (HitComponent :type Primitive%20Component%20Object%20Reference) (OtherActor :type Actor%20Object%20Reference) (OtherComp :type Primitive%20Component%20Object%20Reference) (NormalImpulse :type Vector :default "0, 0, 0") (Hit :type Hit%20Result%20Structure%20%28by%20ref%29))
  (if (!= OtherActor (Variables|Default|GetOwnerCharacter))
    (Utilities|HitFireBall)))

(event OnComponentBeginOverlap(Explode)
  (params (OverlappedComponent :type Primitive%20Component%20Object%20Reference) (OtherActor :type Actor%20Object%20Reference) (OtherComp :type Primitive%20Component%20Object%20Reference) (OtherBodyIndex :type Integer) (bFromSweep :type Boolean) (SweepResult :type Hit%20Result%20Structure%20%28by%20ref%29))
  (if (!= OtherActor (Variables|Default|GetOwnerCharacter))
    (Class|BPICharacterInfo|RecvDamage(Message) OtherActor (/ (Variables|Default|GetDamageValue) 3.0) "(TagName=\"DamageType.Fire\")" (Variables|Default|GetOwnerCharacter))))

(event Custom|Accel
  (bind _projectilemovement (Variables|Default|GetProjectileMovement))
  (Variables|/Script/Engine.MovementComponent|SetVelocity _projectilemovement (* (Variables|/Script/Engine.MovementComponent|GetVelocity (Variables|Default|GetProjectileMovement)) 1.2))
  (Variables|/Script/Engine.ProjectileMovementComponent|SetHomingAccelerationMagnitude (Variables|Default|GetProjectileMovement) (* (Variables|/Script/Engine.ProjectileMovementComponent|GetHomingAccelerationMagnitude _projectilemovement) 1.2)))

(event EventBeginPlay
  (|CallParentFunction)
  (bind _returnvalue (Audio|SpawnSoundatLocation "/Game/SFX/Spell/Fireball/Charge/fireball-whoosh-7-201453_Cue.fireball-whoosh-7-201453_Cue" (Transformation|GetActorLocation) "0, 0, 0" 1.0 1.0 0.0 "/Game/SFX/DefaultAttanuation.DefaultAttanuation" 0))
  (Variables|Default|SetChargeSound _returnvalue)
  (bind _새_트랙_0 (Timeline|타임라인 PlayFromStart)
    (:Update
      (Transformation|SetActorScale3D (Math|Vector|MakeVector _새_트랙_0 _새_트랙_0 _새_트랙_0))
      (Niagara|SetNiagaraVariable(Float) (Variables|Default|GetNS_Fireball) "Scalar" _새_트랙_0)
      (Variables|Default|SetInitialSpeed (* _새_트랙_0 333.0)))))

(event EventProjectileLaunch
  (bind _projectilemovement (Variables|Default|GetProjectileMovement))
  (bind _chargesound (Variables|Default|GetChargeSound))
  (Utilities|FlowControl|Sequence
    (:then_0
      (bind _새_트랙_0 (Timeline|타임라인 Stop)
        (:Update
          (Transformation|SetActorScale3D (Math|Vector|MakeVector _새_트랙_0 _새_트랙_0 _새_트랙_0))
          (Niagara|SetNiagaraVariable(Float) (Variables|Default|GetNS_Fireball) "Scalar" _새_트랙_0)
          (Variables|Default|SetInitialSpeed (* _새_트랙_0 333.0)))))
    (:then_1
      (Transformation|DetachFromActor "KeepWorld" "KeepWorld" "KeepWorld")
      (Variables|/Script/Engine.MovementComponent|SetVelocity _projectilemovement (* (Transformation|GetActorForwardVector) (Variables|Default|GetInitialSpeed)))
      (Variables|/Script/Engine.ProjectileMovementComponent|SetHomingAccelerationMagnitude _projectilemovement 2e+03)
      (Utilities|FlowControl|Delay 9.0)
      (Actor|DestroyActor))
    (:then_2
      (Audio|SpawnSoundatLocation "/Game/SFX/Spell/Fireball/Throw/fire-magic-6-378641_Cue.fire-magic-6-378641_Cue" (Transformation|GetActorLocation) "0, 0, 0" 1.0 1.0 0.0 0 0)
      (Audio|SpawnSoundAttached "/Game/SFX/Spell/Fireball/Woosh/fireball-whoosh-8-201454_Cue.fireball-whoosh-8-201454_Cue" (Variables|Default|GetDefaultSceneRoot) "None" "0, 0, 0" "0, 0, 0" "KeepRelativeOffset" true 1.0 1.0 0.0 "/Game/SFX/DefaultAttanuation.DefaultAttanuation" 0)
      (Utilities|IsValid _chargesound
        (:Is%20Valid
          (Audio|Components|Audio|FadeOut _chargesound 0.5 0.0 "Linear" :!class /Script/Engine.AudioComponent))))
    (:then_3
      (Utilities|Time|SetTimerbyEvent (delegate Custom|Accel) 1.0 true))))

(event EventTick
  (params (DeltaSeconds :type Float%20%28single-precision%29))
  (bind _returnvalue (Transformation|GetActorForwardVector))
  (Niagara|SetNiagaraVariable(Vector3) (Variables|Default|GetNS_Fireball) "NegativeGravityForceDirection" (Math|Vector|Lerp(Vector) _returnvalue (* _returnvalue -1.0) 0.8)))

(fn ConstructionScript)