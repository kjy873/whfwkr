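; Ice spell projectile that adds ice visuals and an optional homing mode to its parent class.
; BeginPlay briefly delays the parent's setup, then activates the ice Niagara effect.
; When flagged as a homing skill, it plays a cast sound and, given a valid target, homes on that actor's root and self-destructs after a timeout.
; PostProcessHit spawns a scaled-down Niagara ice impact; Tick and DebugFunc do nothing.
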(event EventBeginPlay
  (Utilities|FlowControl|Delay 0.1)
  (|CallParentFunction)
  (Components|Activation|Activate (Variables|Default|GetNS_Ice) false)
  (if (Variables|Default|GetbIsHomingSkillMine)
    (Audio|SpawnSoundatLocation "/Game/SFX/Spell/Ice/iced-magic-3-378609_Cue.iced-magic-3-378609_Cue" (Transformation|GetActorLocation) "0, 0, 0" 1.0 1.0 0.0 0 0)
    (if (Utilities|IsValid (Variables|Default|GetTargetActor))
      (Variables|/Script/Engine.ProjectileMovementComponent|SetHomingTargetComponent (Variables|Default|GetProjectileMove) (Variables|/Script/Engine.Actor|GetRootComponent (Variables|Default|GetTargetActor)))
      (Utilities|FlowControl|Delay 6.0)
      (Actor|DestroyActor))))

(event EventTick
  (params (DeltaSeconds :type Float%20%28single-precision%29))
  (Utilities|IsValid (Variables|Default|GetTargetActor)))

(event EventDebugFunc)

(event EventPostProcessHit
  (bind _returnvalue (Niagara|SpawnSystematLocation "/Game/VFX/HitEffect/NS_HitIce.NS_HitIce" (Transformation|GetActorLocation)))
  (Niagara|SetNiagaraVariable(Float) _returnvalue "ScaleMultiplier" 0.5))

(fn ConstructionScript)