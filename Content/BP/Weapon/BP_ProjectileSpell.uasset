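; Spell projectile that picks a homing target for its projectile movement when it spawns.
; On BeginPlay it resolves its owning BP_GameCharacter, falling back to the instigator, then homes on a preset HomingTarget's root component if one is valid.
; Otherwise, a wide box trace from the projectile along the owner's control rotation, ignoring the owner, supplies the hit component as target.
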(event EventBeginPlay
  (bind _homingtarget (Variables|Default|GetHomingTarget))
  (Utilities|IsValid (Variables|Default|GetOwnerCharacter)
    (:Is%20Valid
      _)
    (:Is%20Not%20Valid
      (bind _asbp_game_character (Utilities|Casting|CastToBP_GameCharacter (Game|GetInstigator)))
      (Variables|Default|SetOwnerCharacter _asbp_game_character)))
  (Utilities|IsValid _homingtarget
    (:Is%20Valid
      (Variables|/Script/Engine.ProjectileMovementComponent|SetHomingTargetComponent (Variables|Default|GetProjectileMovement) (Variables|/Script/Engine.Actor|GetRootComponent _homingtarget)))
    (:Is%20Not%20Valid
      (CallFunction|SetHomingTargetbyBoxTrace))))

(event Collision|EventActorBeginOverlap
  (params (OtherActor :type Actor%20Object%20Reference)))

(event EventTick
  (params (DeltaSeconds :type Float%20%28single-precision%29)))

(fn ConstructionScript)

(fn SetHomingTargetbyBoxTrace
  (bind _returnvalue (Transformation|GetActorLocation))
  (bind _ownercharacter (Variables|Default|GetOwnerCharacter))
  (bind _returnvalue_2 (Pawn|GetControlRotation _ownercharacter :!class /Script/Engine.Pawn))
  (bind _outhit (Collision|BoxTraceByChannel _returnvalue (+ _returnvalue (* (Math|Vector|GetForwardVector _returnvalue_2) 5e+03)) "150.000000,1000.000000,1000.000000" _returnvalue_2 "TraceTypeQuery3" false (Utilities|Array|MakeArray (Variables|Default|GetOwnerCharacter)) "None"))
  (if (.bblockinghit _outhit)
    (Variables|/Script/Engine.ProjectileMovementComponent|SetHomingTargetComponent (Variables|Default|GetProjectileMovement) (.hitcomponent _outhit))))