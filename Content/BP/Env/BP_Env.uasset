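; Environment actor that drives a day-night cycle with sun, moon and calendar.
; Date and latitude give solar elevation via declination (computed only at construction and BeginPlay), azimuth maps linearly from time, and the moon light pitches opposite the sun.
; Tick advances time at a toggleable speed, rolling the date over and stepping the 2D moon phase once daily.
; Construction places the 2D or 3D moon and halo, styled through dynamic materials.
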(event EventBeginPlay
  (bind _numofdays (CallFunction|NNumOfDays))
  (bind _declinationofsun (CallFunction|DeclinationOfSun _numofdays))
  (CallFunction|MoonMaterial))

(event Collision|EventActorBeginOverlap
  (params (OtherActor :type Actor%20Object%20Reference)))

(event EventTick
  (params (DeltaSeconds :type Float%20%28single-precision%29))
  (bind (_solarelevationangle _solarazimuthangle) (CallFunction|SolarElevationAngle (stale EventBeginPlay _declinationofsun)))
  (Transformation|SetRelativeRotation (Variables|Default|GetSunLight) (Math|Rotator|MakeRotator 0.0 _solarelevationangle _solarazimuthangle) false false)
  (Transformation|SetRelativeRotation (Variables|Default|GetMoonLight) (Math|Rotator|MakeRotator 0.0 (+ _solarelevationangle 1.8e+02) _solarazimuthangle) false false)
  (Variables|Default_|SetTimeOfDay (+ (Variables|Default_|GetTimeOfDay) (* DeltaSeconds (Variables|Runtime_|GetDaySpeed))))
  (|NextDay))

(event EventSwitchDaySpeed
  (Utilities|FlowControl|FlipFlop
    (:A
      (Variables|Runtime_|SetDaySpeed 2e+01))
    (:B
      (Variables|Runtime_|SetDaySpeed 1.0))))

(fn ConstructionScript
  (bind _moonhaloscale (Variables|Moon|GetMoonHaloScale))
  (bind _usemoon3d (Variables|Moon|GetUseMoon3D))
  (bind _moon3d (Variables|Default|GetMoon3D))
  (bind _moonscale (Variables|Moon|GetMoonScale))
  (bind _returnvalue (* _moonscale 1e+02))
  (Utilities|FlowControl|Sequence
    (:then_0
      (bind _numofdays (CallFunction|NNumOfDays))
      (bind _declinationofsun (CallFunction|DeclinationOfSun _numofdays))
      (bind (_solarelevationangle _solarazimuthangle) (CallFunction|SolarElevationAngle _declinationofsun))
      (Transformation|SetRelativeRotation (Variables|Default|GetSunLight) (Math|Rotator|MakeRotator 0.0 _solarelevationangle (+ _solarazimuthangle (Variables|Default_|GetSunZRotation))) false false)
      (Transformation|SetRelativeRotation (Variables|Default|GetMoonLight) (Math|Rotator|MakeRotator 0.0 (+ _solarelevationangle 1.8e+02) _solarazimuthangle) false false))
    (:then_1
      (Transformation|SetRelativeRotation _moon3d (Math|Conversions|RotationFromXVector (Math|Vector|Normalize (- (Variables|Moon|GetMoonFaceOriginLocation) (Transformation|GetActorLocation)))) false false)
      (Transformation|AddRelativeLocation _moon3d (Math|Vector|MakeVector (Math|Conversions|ToFloat(Integer) (* (Variables|Moon|GetMoonDistanceKm) -100000)) (Math|Conversions|ToFloat(Integer) (* (Variables|Moon|GetMoonLocationHrizontal) 10000)) (Math|Conversions|ToFloat(Integer) (* (Variables|Moon|GetMoonLocationVertical) 10000))) false false)
      (Transformation|SetRelativeScale3D _moon3d (Math|Vector|MakeVector _returnvalue _returnvalue _returnvalue))
      (Transformation|SetRelativeScale3D (Variables|Default|GetMoonHalo) (Math|Vector|MakeVector _moonhaloscale _moonhaloscale _moonhaloscale))
      (Rendering|SetVisibility (Variables|Default|GetMoon3D) _usemoon3d false)
      (Rendering|SetVisibility (Variables|Default|GetMoon2D) (not _usemoon3d) false))
    (:then_2
      (CallFunction|MoonMaterial))))

(fn NNumOfDays
  (LocalVariables|SetDaysInMonth (Utilities|MakeArrayDayinMonth))
  (for _index (range 0 (- (Variables|Default_|GetMonth) 1))
    (LocalVariables|SetCurrentNumOfDays (+ (Utilities|Array|Get(acopy) (LocalVariables|GetDaysInMonth) _index) (LocalVariables|GetCurrentNumOfDays))))
  (bind _output_get (LocalVariables|SetCurrentNumOfDays (+ (LocalVariables|GetCurrentNumOfDays) (Variables|Default_|GetDay) (Math|Integer|SelectInt 0 (Math|Integer|SelectInt 1 0 (== (Math|Float|Fraction (/ (Variables|Default_|GetYear) 4)) 0.0)) (< (Variables|Default_|GetMonth) 3)))))
  (return _output_get))

(fn DeclinationOfSun
  (params (NumOfDays :type Integer))
  (return (* (Math|Trig|Cos(Degrees) (* (/ 3.6e+02 365.0) (+ NumOfDays 10))) 23.44)))

(fn SolarElevationAngle
  (params (DeclinationOfSun :type Float%20%28double-precision%29))
  ;[1 1 1] Elevation
  (LocalVariables|SetDeclination DeclinationOfSun)
  (return (Class|KismetMathLibrary|DegAsin (+ (* (Math|Trig|Sin(Degrees) (Variables|Default_|GetLatitude)) (Math|Trig|Sin(Degrees) (LocalVariables|GetDeclination))) (* (Math|Trig|Cos(Degrees) (Variables|Default_|GetLatitude)) (Math|Trig|Cos(Degrees) (LocalVariables|GetDeclination)) (Math|Trig|Cos(Degrees) (* (/ (Variables|Default_|GetTimeOfDay) 1e+02) 15.0))))) (+ (Math|Float|MapRangeClamped (Variables|Default_|GetTimeOfDay) 0.0 2.4e+03 0.0 3.6e+02) 1.8e+02)))

(fn MoonMaterial
  (Utilities|FlowControl|Sequence
    (:then_0
      (if (Variables|Moon|GetUseMoon3D)
        (bind _returnvalue (Rendering|Material|CreateDynamicMaterialInstance (Variables|Default|GetMoon3D) 0 0 "None" :!class /Script/Engine.PrimitiveComponent))
        (Variables|MoonMaterial|SetDMI_Moon3D _returnvalue)
        (Rendering|Material|SetVectorParameterValue (Variables|MoonMaterial|GetDMI_Moon3D) "BaseColor" (Variables|MoonMaterial|GetMoon3DBaseColor) :!class /Script/Engine.MaterialInstanceDynamic)
        (Rendering|Material|SetVectorParameterValue (Variables|MoonMaterial|GetDMI_Moon3D) "EdgeColor" (Variables|MoonMaterial|GetMoon3DEdgeColor) :!class /Script/Engine.MaterialInstanceDynamic)
        (Rendering|Material|SetScalarParameterValue (Variables|MoonMaterial|GetDMI_Moon3D) "BaseSaturation" (Variables|MoonMaterial|GetMoon3DBaseSaturation) :!class /Script/Engine.MaterialInstanceDynamic)
        (Rendering|Material|SetScalarParameterValue (Variables|MoonMaterial|GetDMI_Moon3D) "BaseIntensity" (Variables|MoonMaterial|GetMoon3DBaseIntensity) :!class /Script/Engine.MaterialInstanceDynamic)
        (Rendering|Material|SetScalarParameterValue (Variables|MoonMaterial|GetDMI_Moon3D) "EdgeIntensity" (Variables|MoonMaterial|GetMoon3DEdgeIntensity) :!class /Script/Engine.MaterialInstanceDynamic)
        (Rendering|Material|SetScalarParameterValue (Variables|MoonMaterial|GetDMI_Moon3D) "EdgeDensity" (Variables|MoonMaterial|GetMoon3DEdgeDensity) :!class /Script/Engine.MaterialInstanceDynamic)
        (Rendering|Material|SetScalarParameterValue (Variables|MoonMaterial|GetDMI_Moon3D) "EdgeDensity" (Variables|MoonMaterial|GetMoon3DUvs) :!class /Script/Engine.MaterialInstanceDynamic)
        (else
          (bind _returnvalue_2 (Rendering|Material|CreateDynamicMaterialInstance (Variables|Default|GetMoon2D) 0 "/Game/BP/Env/Material/M_Moon2D.M_Moon2D" "None" :!class /Script/Engine.PrimitiveComponent))
          (Variables|MoonMaterial|SetDMI_Moon2D _returnvalue_2)
          (Rendering|Material|SetVectorParameterValue (Variables|MoonMaterial|GetDMI_Moon2D) "BaseColor" (Variables|MoonMaterial|GetMoon2D_BaseColor) :!class /Script/Engine.MaterialInstanceDynamic)
          (Rendering|Material|SetVectorParameterValue (Variables|MoonMaterial|GetDMI_Moon2D) "EdgeColor" (Variables|MoonMaterial|GetMoon2D_EdgeColor) :!class /Script/Engine.MaterialInstanceDynamic)
          (Rendering|Material|SetScalarParameterValue (Variables|MoonMaterial|GetDMI_Moon2D) "BaseSaturation" (Variables|MoonMaterial|GetMoon2D_BaseSaturation) :!class /Script/Engine.MaterialInstanceDynamic)
          (Rendering|Material|SetScalarParameterValue (Variables|MoonMaterial|GetDMI_Moon2D) "BaseIntensity" (Variables|MoonMaterial|GetMoon2D_BaseIntensity) :!class /Script/Engine.MaterialInstanceDynamic)
          (Rendering|Material|SetScalarParameterValue (Variables|MoonMaterial|GetDMI_Moon2D) "EdgeSaturation" (Variables|MoonMaterial|GetMoon2D_EdgeSaturation) :!class /Script/Engine.MaterialInstanceDynamic)
          (Rendering|Material|SetScalarParameterValue (Variables|MoonMaterial|GetDMI_Moon2D) "EdgeIntensity" (Variables|MoonMaterial|GetMoon2D_EdgeIntensity) :!class /Script/Engine.MaterialInstanceDynamic)
          (Rendering|Material|SetScalarParameterValue (Variables|MoonMaterial|GetDMI_Moon2D) "AnimationPhase" (Math|Float|Clamp(Float) (Variables|MoonMaterial|GetMoon2DAnimationPhase) 0.0 32.0) :!class /Script/Engine.MaterialInstanceDynamic)
          (Rendering|Material|SetScalarParameterValue (Variables|MoonMaterial|GetDMI_Moon2D) "RotationAngle" (Math|Float|Clamp(Float) (Variables|MoonMaterial|GetMoon2DRotationAngle) 0.0 3.6e+02) :!class /Script/Engine.MaterialInstanceDynamic))))
    (:then_1
      (bind _returnvalue_3 (Rendering|Material|CreateDynamicMaterialInstance (Variables|Default|GetMoonHalo) 0 0 "None" :!class /Script/Engine.PrimitiveComponent))
      (Variables|MoonMaterial|SetDMI_MoonHalo _returnvalue_3)
      (Rendering|Material|SetVectorParameterValue (Variables|MoonMaterial|GetDMI_MoonHalo) "BaseColor" (Variables|MoonMaterial|GetMoonHaloBaseColor) :!class /Script/Engine.MaterialInstanceDynamic)
      (Rendering|Material|SetScalarParameterValue (Variables|MoonMaterial|GetDMI_MoonHalo) "Radius" (Variables|MoonMaterial|GetMoonHaloRadius) :!class /Script/Engine.MaterialInstanceDynamic)
      (Rendering|Material|SetScalarParameterValue (Variables|MoonMaterial|GetDMI_MoonHalo) "Density" (Variables|MoonMaterial|GetMoonHaloDensity) :!class /Script/Engine.MaterialInstanceDynamic)
      (Rendering|Material|SetScalarParameterValue (Variables|MoonMaterial|GetDMI_MoonHalo) "Saturation" (Variables|MoonMaterial|GetMoonHaloSaturation) :!class /Script/Engine.MaterialInstanceDynamic)
      (Rendering|Material|SetScalarParameterValue (Variables|MoonMaterial|GetDMI_MoonHalo) "Intensity" (Variables|MoonMaterial|GetMoonHaloIntensity) :!class /Script/Engine.MaterialInstanceDynamic))))