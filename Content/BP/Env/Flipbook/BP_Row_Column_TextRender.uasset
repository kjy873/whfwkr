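; Construction-script actor in the Flipbook environment folder that builds a numbered grid of rows and columns over a backing plane.
; A nested loop adds a centered TextRender per cell with a running number, alternating color by row parity.
; A static mesh plane with the assigned material is then centered and scaled to the row and column counts, with shadows off.
; Finally, the whole actor is uniformly scaled, and the event graph is empty.
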(event EventBeginPlay)

(event Collision|EventActorBeginOverlap
  (params (OtherActor :type Actor%20Object%20Reference)))

(event EventTick
  (params (DeltaSeconds :type Float%20%28single-precision%29)))

(fn ConstructionScript
  (bind _odd_numberedrows (Variables|Number|GetOdd-NumberedRows))
  (bind _even_numberedrows (Variables|Number|GetEven-NumberedRows))
  (bind _textscale (Variables|Transform_|GetTextScale))
  (bind _scale (Variables|Plane_|GetScale))
  (bind (_b _g _r _a) (Math|Color|BreakColor _even_numberedrows))
  (bind (_b_2 _g_2 _r_2 _a_2) (Math|Color|BreakColor _odd_numberedrows))
  (Utilities|FlowControl|Sequence
    (:then_0
      ;[0 0 0] Text Render
      (for _index (range 0 (- (Variables|Number|GetColNumber) 1)) :!label _label
        (bind _output_get (LocalVariables|SetColIndex _index))
        (LocalVariables|SetColLocation (* _output_get (Variables|Transform_|GetColRange)))
        (LocalVariables|SetRowLocation (* (Variables|Transform_|GetRowRange) (LocalVariables|GetRowIndex)))
        (bind _returnvalue (AddComponent|AddTextRenderComponent false (Math|Transform|MakeTransform (Math|Vector|MakeVector -2.0 (LocalVariables|GetColLocation) (* (LocalVariables|GetRowLocation) -1.0)) "0.000000,180.000000,0.000000" (Math|Vector|MakeVector _textscale _textscale _textscale))))
        (Variables|Default|SetRef_TextReder _returnvalue)
        (bind _output_get_2 (LocalVariables|SetTextNumber (+ (LocalVariables|GetTextNumber) 1)))
        (Rendering|Components|TextRender|SetText (Variables|Default|GetRef_TextReder) (Utilities|Text|ToText(Integer) _output_get_2))
        (Rendering|Components|TextRender|SetTextRenderColor (Variables|Default|GetRef_TextReder) (select (== (Math|Integer|%(Integer) (LocalVariables|GetRowIndex) 2) 0) (Math|Color|MakeColor _b_2 _g_2 _r_2 _a_2) (Math|Color|MakeColor _b _g _r _a)))
        (Rendering|Components|TextRender|SetHorizontalAlignment (Variables|Default|GetRef_TextReder) "EHTA_Center")
        (Class|TextRenderComponent|SetVerticalAlignment (Variables|Default|GetRef_TextReder) "EVRTA_TextCenter"))
      (if (not (<= (- (Variables|Number|GetRowNumber) 1) (LocalVariables|GetRowIndex)))
        (Math|Integer|IncrementInt (LocalVariables|GetRowIndex)
          (:%20%20
            (goto _label)))))
    (:then_1
      ;[0 0 0] Plane
      (bind _returnvalue_2 (AddComponent|AddStaticMeshComponent false))
      (bind _output_get_3 (Variables|Default|SetRef_Plane _returnvalue_2))
      (Rendering|Material|SetMaterial _output_get_3 0 (Variables|Plane_|GetMaterial))
      (Transformation|SetRelativeTransform (Variables|Default|GetRef_Plane) (Math|Transform|MakeTransform (Math|Vector|MakeVector -1.0 (/ (* (LocalVariables|GetColIndex) (Variables|Transform_|GetColRange)) 2.0) (* (/ (* (Variables|Transform_|GetRowRange) (LocalVariables|GetRowIndex)) 2.0) -1.0)) "0.000000,90.000000,90.000000" (Math|Vector|MakeVector (Math|Conversions|ToFloat(Integer) (+ (LocalVariables|GetColIndex) 1)) (Math|Conversions|ToFloat(Integer) (+ (LocalVariables|GetRowIndex) 1)) 1.0)) false false)
      (Rendering|SetCastShadow (Variables|Default|GetRef_Plane) false))
    (:then_2
      ;[0 0 0] Actor Scale
      (Transformation|SetActorScale3D (Math|Vector|MakeVector _scale _scale _scale)))))