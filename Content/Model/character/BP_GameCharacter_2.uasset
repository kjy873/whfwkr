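; Game character Blueprint that holds health, mana, stamina, experience and level stats.
; Tick computes ground speed and movement direction relative to control yaw, and pushes stat values to the controller's display functions every frame.
; Add and subtract functions cap values at max or zero, though mana has no subtract.
; AddExp levels up at max EXP, discarding overflow, and LevelUp only refreshes the level display, also set on BeginPlay.
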(event EventBeginPlay
  (Class|BPStats|UpdateLevelDisplay(Message) (Pawn|GetController) (Variables|Default|GetCharacterLevel)))

(event Collision|EventActorBeginOverlap
  (params (OtherActor :type Actor%20Object%20Reference)))

(event EventTick
  (params (DeltaSeconds :type Float%20%28single-precision%29))
  (bind _returnvalue (Pawn|GetController))
  (Variables|Default|SetGroundSpeed (Math|Vector|VectorLengthXY (Transformation|GetVelocity)))
  (Variables|Default|SetMoveDirectionAngle (Class|KismetAnimationLibrary|CalculateDirection (Transformation|GetVelocity) (Math|Rotator|MakeRotator 0.0 0.0 (.yaw (Pawn|GetControlRotation :!class /Script/Engine.Pawn)))))
  (Class|BPStats|UpdateHealthDisplay(Message) _returnvalue (Variables|Default|GetHP) (Variables|Default|GetMaxHP))
  (Class|BPStats|UpdateManaDisplay(Message) _returnvalue (Variables|Default|GetMana) (Variables|Default|GetMaxMana))
  (Class|BPStats|UpdateStaminaDisplay(Message) _returnvalue (Variables|Default|GetStamina) (Variables|Default|GetMaxStamina))
  (Class|BPStats|UpdateExpDisplay(Message) _returnvalue (Variables|Default|GetEXP) (Variables|Default|GetMaxEXP)))

(fn ConstructionScript)

(fn AddExp
  (params (Value :type Float%20%28double-precision%29))
  (bind _output_get (Variables|Default|SetEXP (+ (Variables|Default|GetEXP) Value)))
  (if (>= _output_get (Variables|Default|GetMaxEXP))
    (Math|Integer|IncrementInt (Variables|Default|GetCharacterLevel)
      (:%20%20
        (CallFunction|LevelUp)
        (Variables|Default|SetEXP 0.0)))))

(fn SubtractStamina
  (params (Value :type Float%20%28double-precision%29))
  (bind _output_get (Variables|Default|SetStamina (- (Variables|Default|GetStamina) Value)))
  (if (< _output_get 0.0)
    (Variables|Default|SetStamina 0.0)))

(fn AddStamina
  (params (Value :type Float%20%28double-precision%29))
  (bind _output_get (Variables|Default|SetStamina (+ (Variables|Default|GetStamina) Value)))
  (if (> _output_get (Variables|Default|GetMaxStamina))
    (Variables|Default|SetStamina (Variables|Default|GetMaxStamina))))

(fn SubtractHealth
  (params (Value :type Float%20%28double-precision%29))
  (bind _output_get (Variables|Default|SetHP (- (Variables|Default|GetHP) Value)))
  (if (< _output_get 0.0)
    (Variables|Default|SetHP 0.0)))

(fn AddHealth
  (params (Value :type Float%20%28double-precision%29))
  (bind _output_get (Variables|Default|SetHP (+ (Variables|Default|GetHP) Value)))
  (if (>= _output_get (Variables|Default|GetMaxHP))
    (Variables|Default|SetHP (Variables|Default|GetMaxHP))))

(fn LevelUp
  (Class|BPStats|UpdateLevelDisplay(Message) (Pawn|GetController) (Variables|Default|GetCharacterLevel)))

(fn AddMana
  (params (Value :type Float%20%28double-precision%29))
  (bind _output_get (Variables|Default|SetMana (+ (Variables|Default|GetMana) Value)))
  (if (> _output_get (Variables|Default|GetMaxMana))
    (Variables|Default|SetMana (Variables|Default|GetMaxMana))))