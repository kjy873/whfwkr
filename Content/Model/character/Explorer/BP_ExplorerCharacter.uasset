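; BP_ExplorerCharacter is the playable Explorer character, handling movement, jump and attack through Enhanced Input actions.
; Move input drives movement along forward and right vectors from control yaw, while Tick turns the MoveDirection component to that yaw plus MoveDirectionAngle.
; Left click plays the sped-up Explorer_Attack montage, followed by a Delay that leads nowhere.
; Jump input calls Jump and sets a Jump flag, which this graph never resets.
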(event Input|EnhancedActionEvents|EnhancedInputActionIA_Default_Move
  (params (ActionValue :type Vector%202D%20Structure) (ElapsedSeconds :type Float%20%28double-precision%29) (TriggeredSeconds :type Float%20%28double-precision%29) (InputAction :type Input%20Action%20Object%20Reference :default "/Game/BP/Input_Action/IA_Default_Move.IA_Default_Move"))
  (bind _returnvalue (Pawn|GetControlRotation :!class /Script/Engine.Pawn))
  (bind _returnvalue_2 (Math|Rotator|MakeRotator 0.0 0.0 (.yaw _returnvalue)))
  (Pawn|Input|AddMovementInput (Math|Vector|GetForwardVector _returnvalue_2) (.x ActionValue) false)
  (Pawn|Input|AddMovementInput (Math|Vector|GetRightVector _returnvalue_2) (.y ActionValue) false))

(event Input|EnhancedActionEvents|EnhancedInputActionIA_LeftClick
  (params (ActionValue :type Boolean) (ElapsedSeconds :type Float%20%28double-precision%29) (TriggeredSeconds :type Float%20%28double-precision%29) (InputAction :type Input%20Action%20Object%20Reference :default "/Game/BP/Input_Action/IA_LeftClick.IA_LeftClick"))
  (Animation|Montage|PlayMontage (Variables|Character|GetMesh) "/Game/Model/character/Explorer/Animation/Explorer_Attack.Explorer_Attack" 1.5 0.0 "Default"
    (:then
      (Utilities|FlowControl|Delay 0.3))))

(event Input|EnhancedActionEvents|EnhancedInputActionIA_Jump
  (params (ActionValue :type Boolean) (ElapsedSeconds :type Float%20%28double-precision%29) (TriggeredSeconds :type Float%20%28double-precision%29) (InputAction :type Input%20Action%20Object%20Reference :default "/Game/BP/Input_Action/IA_Jump.IA_Jump"))
  (Character|Jump)
  (Variables|Default|SetJump? true))

(event EventBeginPlay
  (|CallParentFunction) ; 지금 이 노드는 비활성 상태입니다. \n핀을 끌어서 다른 노드를 연결하면 활성화됩니다.
)

(event Collision|EventActorBeginOverlap
  (params (OtherActor :type Actor%20Object%20Reference))
  (|CallParentFunction OtherActor) ; 지금 이 노드는 비활성 상태입니다. \n핀을 끌어서 다른 노드를 연결하면 활성화됩니다.
)

(event EventTick
  (params (DeltaSeconds :type Float%20%28single-precision%29))
  (|CallParentFunction DeltaSeconds)
  (Transformation|SetWorldRotation (Variables|Default|GetMoveDirection) (Math|Rotator|MakeRotator 0.0 0.0 (+ (.yaw (Pawn|GetControlRotation :!class /Script/Engine.Pawn)) (Variables|Default|GetMoveDirectionAngle))) false false))

(fn ConstructionScript
  (|CallParentFunction))