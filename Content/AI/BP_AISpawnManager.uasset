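; AI spawn manager that sets up regions, each with hard and soft activation states, at game start.
; BeginPlay gets the current world, registers player 0's character in PlayerActors, then calls GenerateRegion and starts the update timer only if generation succeeds.
; Region generation and update logic are defined outside this graph; Tick is empty.
; An unconnected debug chain would print each region's activation states after a delay.
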(event EventBeginPlay
  (bind _returnvalue (Game|GetPlayerCharacter 0))
  (Class|AISpawnManager|GetCurrentWorld)
  (Utilities|IsValid _returnvalue
    (:Is%20Valid
      (Utilities|Array|AddUnique (Variables|Default|GetPlayerActors) _returnvalue))
    (:Is%20Not%20Valid
      _))
  (bind _returnvalue_2 (Class|AISpawnManager|GenerateRegion))
  (if _returnvalue_2
    (Class|AISpawnManager|SetUpdateTimer)))

(event EventTick
  (params (DeltaSeconds :type Float%20%28single-precision%29)))

(fn ConstructionScript)