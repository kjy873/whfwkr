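; BP_NPC2 is an AI character that punches a target and drops experience orbs when hit by a player character.
; Attack sphere-traces nearby pawns, then applies damage and plays a punch montage if the given target is found.
; RecvDamage from a BP_GameCharacter spawns scattered orbs targeting the instigator, scaled by level, and calls DestroyActor inside that loop with no health check.
; AnyDamage only prints a debug string.
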(event Custom|OnDamaged
  (params (Value :type Float%20%28double-precision%29) (DamageType :type Gameplay%20Tag%20Structure) (Subject :type Actor%20Object%20Reference)))

(event EventBeginPlay)

(event Collision|EventActorBeginOverlap
  (params (OtherActor :type Actor%20Object%20Reference)))

(event EventTick
  (params (DeltaSeconds :type Float%20%28single-precision%29)))

(event EventAttack
  (params (TargetAction :type Actor%20Object%20Reference))
  (bind _returnvalue (Transformation|GetActorLocation))
  (bind (_outhits _returnvalue_2) (Collision|MultiSphereTraceForObjects _returnvalue _returnvalue 2e+02 (Utilities|Array|MakeArray "ObjectTypeQuery3") false 0 "None"))
  (if _returnvalue_2
    (bind _array_element (Utilities|Array|ForEachLoopwithBreak _outhits :!label _label)
      (:LoopBody
        (if (== TargetAction (.HitActor (Collision|BreakHitResult _array_element)))
          (Game|Damage|ApplyDamage (.HitActor (Collision|BreakHitResult _array_element)) 1e+01 0 0)
          (Animation|Montage|PlayMontage (Variables|Character|GetMesh) "/Game/Characters/AI/MonsterAniMation/Punching_Montage.Punching_Montage"
            (:then
              (goto _label Break))))))))

(event Game|Damage|EventAnyDamage
  (params (Damage :type Float%20%28single-precision%29) (DamageType :type Damage%20Type%20Object%20Reference) (InstigatedBy :type Controller%20Object%20Reference) (DamageCauser :type Actor%20Object%20Reference))
  (Development|PrintString "Duch"))

(event EventRecvDamage
  (params (Value :type Float%20%28double-precision%29) (DamageType :type Gameplay%20Cue%20Tag%20Structure) (Instigator :type Pawn%20Object%20Reference))
  (bind _returnvalue (Math|Random|RandomFloatinRange -3e+01 3e+01))
  (bind _asbp_game_character (Utilities|Casting|CastToBP_GameCharacter Instigator)
    (:then
      (for _index (range 0 (- (* (.level (Variables|Default|GetAttributes)) 2) 1))
        (Game|SpawnActorfromClass "/Game/BP/Actors/BP_ExpOrb.BP_ExpOrb_C" (Math|Transform|MakeTransform (+ (Transformation|GetActorLocation) (Math|Vector|MakeVector _returnvalue _returnvalue _returnvalue)) "0, 0, 0" "1.000000,1.000000,1.000000") "Undefined" "MultiplyWithRoot" 0 _asbp_game_character 0)
        (Actor|DestroyActor)))
    (:CastFailed
      (Development|PrintString "AI Damaged :: Instigator is not GameCharacter"))))

(fn ConstructionScript)

(fn GetAnimatedMesh
  (return 0))

(fn IsCharacter
  (return false))