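; BP_NPC is an AI character blueprint with a simple area-checked attack and a placeholder damage reaction.
; The Attack event runs a sphere trace for Pawns around the NPC and, if the passed target is among the hits, applies damage to it, calls Play Montage on the mesh and exits the loop.
; Taking any damage only prints a debug string, with no health handling in this graph.
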(event EventBeginPlay)

(event Collision|EventActorBeginOverlap
  (params (OtherActor :type Actor%20Object%20Reference)))

(event EventTick
  (params (DeltaSeconds :type Float%20%28single-precision%29)))

(event EventAttack
  (params (TargetAction :type Actor%20Object%20Reference))
  (bind _returnvalue (Transformation|GetActorLocation))
  (bind (_outhits _returnvalue_2) (Collision|MultiSphereTraceForObjects _returnvalue _returnvalue 2e+02 (Utilities|Array|MakeArray "ObjectTypeQuery3") false 0 "None"))
  (if _returnvalue_2
    (bind _array_element (Utilities|Array|ForEachLoopwithBreak _outhits :!label _label)
      (:LoopBody
        (if (== TargetAction (.HitActor (Collision|BreakHitResult _array_element)))
          (Game|Damage|ApplyDamage (.HitActor (Collision|BreakHitResult _array_element)) 1e+01 0 0)
          (Animation|Montage|PlayMontage (Variables|Character|GetMesh) 0
            (:then
              (goto _label Break))))))))

(event Game|Damage|EventAnyDamage
  (params (Damage :type Float%20%28single-precision%29) (DamageType :type Damage%20Type%20Object%20Reference) (InstigatedBy :type Controller%20Object%20Reference) (DamageCauser :type Actor%20Object%20Reference))
  (Development|PrintString "Duch"))

(fn ConstructionScript)