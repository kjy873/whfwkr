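; BP_Portal_1 is a level-transition portal that sends the player to GameMap.
; When a BP_Knight_2 actor begins overlapping the Triger component, it opens that level by name immediately.
; Every tick, ChangeTimerMap counts a Time variable down toward zero, but the countdown does not gate the transition.
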(event OnComponentBeginOverlap(Triger)
  (params (OverlappedComponent :type Primitive%20Component%20Object%20Reference) (OtherActor :type Actor%20Object%20Reference) (OtherComp :type Primitive%20Component%20Object%20Reference) (OtherBodyIndex :type Integer) (bFromSweep :type Boolean) (SweepResult :type Hit%20Result%20Structure%20%28by%20ref%29))
  (Utilities|Casting|CastToBP_Knight_2 OtherActor)
  (Game|OpenLevel(byName) "GameMap"))

(event Custom|ChangeTimerMap
  (bind _output_get (Variables|Default|Settime (Math|Float|Clamp(Float) (- (Variables|Default|Gettime) (Utilities|Time|GetWorldDeltaSeconds)) 0.0 (Variables|Default|Gettime)))))

(event EventTick
  (params (DeltaSeconds :type Float%20%28single-precision%29))
  (CallFunction|ChangeTimerMap))

(fn ConstructionScript)